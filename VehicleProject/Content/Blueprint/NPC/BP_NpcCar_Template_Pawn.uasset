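; NPC car pawn template that drives itself along the nearest BP_Path spline, chosen at BeginPlay.
; Each Tick, it steers toward a spline point projected ahead along the tangent, with look-ahead growing with speed.
; Braking samples a further point from that target to anticipate bends, and releases at low speed.
; The steering yaw error also sets a target speed that switches throttle between forward and reverse input.
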(event `self.ReceiveBeginPlay`
  (bind _outactors (`GameplayStatics.GetAllActorsOfClass` "/Game/Blueprint/NPC/BP_Path.BP_Path_C"))
  (bind _spline_actor (`self.Find Nearest Spline` _outactors))
  (bind _output_get (set `self.Default Spline` _spline_actor))
  (set `self.SplineActor` _output_get))

(event `self.ReceiveTick`
  (params (DeltaSeconds :type "Float (single-precision)"))
  (bind _vehiclemovementcomponent (`self.VehicleMovementComponent`))
  (`/Engine/EditorBlueprintResources/StandardMacros.IsValid` (`self.SplineActor`)
    (:`Is Valid`
      (`|ExecutionSequence`
        (:`then_0`
          (bind _steering (`self.Calc Steering` (`self.SplineActor`)))
          (`ChaosVehicleMovementComponent.SetSteeringInput` (`self.VehicleMovementComponent`) _steering)
          (bind _brake_value (`self.Calc Brake` (`self.SplineActor`) (`self.OffsetTangentLocation`)))
          (`ChaosVehicleMovementComponent.SetBrakeInput` (`self.VehicleMovementComponent`) _brake_value))
        (:`then_1`
          (set `self.TangentSpeed` (`KismetMathLibrary.MapRangeClamped` (`KismetMathLibrary.Abs` (`self.YawDelta`)) 30.0 5.0 (`self.MinSpeed`) (`self.MaxSpeed`)))
          (if (< (`ChaosVehicleMovementComponent.GetForwardSpeedMPH` (`self.VehicleMovementComponent`)) (`self.TangentSpeed`))
            (`ChaosVehicleMovementComponent.SetThrottleInput` _vehiclemovementcomponent 0.3)
            (else
              (`ChaosVehicleMovementComponent.SetThrottleInput` _vehiclemovementcomponent -1.0))))))))

(fn `Calc Brake`
  (params (Spline :type "/Game/Blueprint/NPC/BP_Path Object Reference") (OriginLocation :type "Vector Structure"))
  (returns (`Brake Value` :type "Float (double-precision)"))
  (locals (`Brake Input` :type "Float (double-precision)"))
  (bind _spline (`/Game/Blueprint/NPC/BP_Path.Spline` Spline))
  (bind _returnvalue (`ChaosVehicleMovementComponent.GetForwardSpeedMPH` (`self.VehicleMovementComponent`)))
  (bind (_returnvalue_roll _returnvalue_pitch _returnvalue_yaw) (`KismetMathLibrary.BreakRotator` (`KismetMathLibrary.NormalizedDeltaRotator` (`KismetMathLibrary.FindLookAtRotation` (`self.K2_GetActorLocation`) (`SplineComponent.FindLocationClosestToWorldLocation` _spline (+ OriginLocation (* (`KismetMathLibrary.Normal` (`SplineComponent.FindTangentClosestToWorldLocation` _spline OriginLocation "World")) (* (`KismetMathLibrary.FClamp` _returnvalue 1.0 _returnvalue) 50.0))) "World")) (`self.K2_GetActorRotation`))))
  (if (`self.DebugBrake`)
    (set `local.Brake Input` (`KismetMathLibrary.MapRangeClamped` (+ (`KismetMathLibrary.Abs` _returnvalue_yaw) (/ (`KismetMathLibrary.Abs` (`self.YawDelta`)) 4.0)) 15.0 35.0 0.0 1.0))
    (if (<= (`ChaosVehicleMovementComponent.GetForwardSpeedMPH` (`self.VehicleMovementComponent`)) 5.0)
      (set `local.Brake Input` 0.0))
    (return (`local.Brake Input`))))

(fn `Calc Steering`
  (params (Spline :type "/Game/Blueprint/NPC/BP_Path Object Reference"))
  (returns (Steering :type "Float (double-precision)"))
  (bind _returnvalue (`self.K2_GetActorLocation`))
  (bind _spline (`/Game/Blueprint/NPC/BP_Path.Spline` Spline))
  (bind _returnvalue_2 (`SplineComponent.FindLocationClosestToWorldLocation` _spline (+ (* (`KismetMathLibrary.Normal` (`SplineComponent.FindTangentClosestToWorldLocation` _spline (`self.K2_GetActorLocation`) "World")) (+ 250.0 (* (`ChaosVehicleMovementComponent.GetForwardSpeedMPH` (`self.VehicleMovementComponent`)) 10.0))) _returnvalue) "World"))
  (bind (_returnvalue_roll _returnvalue_pitch _returnvalue_yaw) (`KismetMathLibrary.BreakRotator` (`KismetMathLibrary.NormalizedDeltaRotator` (`KismetMathLibrary.FindLookAtRotation` _returnvalue _returnvalue_2) (`self.K2_GetActorRotation`))))
  (bind _output_get (set `self.OffsetTangentLocation` _returnvalue_2))
  (if (`self.DebugSteering`)
    (`KismetSystemLibrary.DrawDebugSphere` _output_get 25.0 12 (struct :`R` 1.0 :`A` 1.0) 0.0 1.0)
    (`KismetSystemLibrary.DrawDebugArrow` _returnvalue _output_get 1.0 (struct :`R` 1.0 :`A` 1.0) 0.0 10.0)
    (set `self.YawDelta` _returnvalue_yaw)
    (return (`KismetMathLibrary.MapRangeClamped` _returnvalue_yaw -15.0 15.0 -1.0 1.0))))

(fn `Find Nearest Spline`
  (params (`Spline Actors` :type "Array of /Game/Blueprint/NPC/BP_Path Object Reference"))
  (returns (`Spline Actor` :type "/Game/Blueprint/NPC/BP_Path Object Reference"))
  (bind _returnvalue (`self.K2_GetActorLocation`))
  (set `self.Distance` 0.0)
  (for (_array_element _array_index) `Spline Actors`
    (if (== _array_index 0)
      (bind _returnvalue_2 (`KismetMathLibrary.Vector_Distance` (`SplineComponent.FindLocationClosestToWorldLocation` (`/Game/Blueprint/NPC/BP_Path.Spline` _array_element) _returnvalue "World") _returnvalue))
      (set `self.Distance` _returnvalue_2 :!label _label)
      (set `self.Nearest Spline` _array_element)
      (elif (< _returnvalue_2 (`self.Distance`))
        (goto _label))))
  (return (`self.Nearest Spline`)))

(fn `Init Mesh`
  (params (`New Mesh` :type "StaticMesh Object Reference"))
  (`StaticMeshComponent.SetStaticMesh` (`self.Chassis`) `New Mesh`))

(fn `Set Throttle`
  (params (`Throttle Value` :type "Float (double-precision)"))
  (`ChaosVehicleMovementComponent.SetThrottleInput` (`self.VehicleMovementComponent`) `Throttle Value`))

(fn `UserConstructionScript`)